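; MouseInteractManager is the mouse-driven camera and interaction actor for a product viewer, extending a parent manager class.
; BeginPlay makes it the view target and shows the cursor; Tick accumulates zoom and converts mouse delta into swipe speed.
; Left-click traces for a tagged model, falling back to the previous hit location, and drives rotation and interest-point logic.
; Right-click toggles translation, saving the actor's location on release.
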(event EventBeginPlay
  (bind _returnvalue (Game|GetPlayerController 0))
  (|CallParentFunction)
  (Utilities|FlowControl|Sequence
    (:then_0
      ;[1 1 1] Setup the Camera
      (Game|Player|SetViewTargetwithBlend (Game|GetPlayerController 0) self 0.0 "VTBlend_Linear" 0.0 false))
    (:then_1
      ;[1 1 1] Setup the Input modes
      (Input|EnableInput _returnvalue)
      (Variables|/Script/Engine.PlayerController|SetbEnableClickEvents _returnvalue true)
      (Variables|/Script/Engine.PlayerController|SetbShowMouseCursor _returnvalue true)
      (Input|SetIgnoreLookInput _returnvalue true))))

(event EventTick
  (params (DeltaSeconds :type Float%20%28single-precision%29))
  (bind _returnvalue (Game|GetPlayerController 0))
  (bind _swipe_scale (Variables|Default|GetSwipe_Scale))
  (bind (_deltax _deltay) (Class|PlayerController|GetInputMouseDelta _returnvalue))
  (Utilities|FlowControl|Sequence
    (:then_0
      ;[1 1 1] Get Zoom
      (Variables|Default|SetCameraZoom (+ (* (Variables|Default|GetCameraZoomScale) (Class|Actor|GetInputAxisKeyValue)) (Variables|Default|GetCameraZoom))))
    (:then_1
      ;[1 1 1] Get Rotation
      (Variables|Default|SetInteractSwipeSpeed (Math|Vector2D|MakeVector2D (* _deltax _swipe_scale) (* _deltay _swipe_scale))))
    (:then_2
      (|CallParentFunction DeltaSeconds))))

(event Input|MouseEvents|LeftMouseButton
  (params (Key :type Key%20Structure))
  (bind _returnvalue (Game|GetPlayerController 0))
  (bind (_locationx _locationy) (Game|Player|GetMousePosition _returnvalue))
  (bind _returnvalue_2 (Math|Vector2D|MakeVector2D _locationx _locationy))
  ;[1 1 1] Rotate
  (:Pressed
    (Variables|Default|SetStartInteractingLocation _returnvalue_2)
    (CallFunction|GetHitLocModel false)
    (CallFunction|SetReversedRotation))
  (:Released
    (Variables|Default|SetStopInteractingLocation _returnvalue_2)
    (CallFunction|SetInterestPoint)))

(event Input|MouseEvents|RightMouseButton
  (params (Key :type Key%20Structure))
  ;[1 1 1] Translate
  (:Pressed
    (Variables|Default|SetIsTranslating true))
  (:Released
    (Variables|Default|SetIsTranslating false)
    (Variables|Default|SetPreviousTraceHitLocation (Transformation|GetActorLocation self))))

(fn ConstructionScript
  (|CallParentFunction))

(fn GetHitLocModel
  (params (ExcludeModels :type Boolean))
  (bind _returnvalue (Game|GetPlayerController 0))
  (bind _array (Utilities|Array|MakeArray "ObjectTypeQuery1" "ObjectTypeQuery2"))
  (bind (_hitresult _returnvalue_2) (Class|PlayerController|GetHitResultUnderCursorforObjects _returnvalue _array true))
  (bind (_bblockinghit _binitialoverlap _time _distance _location _impactpoint _normal _impactnormal _physmat _hitactor) (Collision|BreakHitResult _hitresult))
  (if _returnvalue_2
    (if (!= (Utilities|Array|FindItem (Variables|/Script/Engine.Actor|GetTags _hitactor) (Utilities|Array|Get(acopy) (Variables|Default|GetInteractiveTag))) -1)
      (Variables|Default|SetTraceHitLocation _location)
      (Variables|Default|SetHitModel _hitactor)
      (else
        (Variables|Default|SetTraceHitLocation (Variables|Default|GetPreviousTraceHitLocation) :!label _label)))
    (else
      (goto _label)))
  (bind _out (|CallParentFunction false))
  (return _out "0, 0, 0"))