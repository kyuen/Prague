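; VR interaction manager for a product viewer: right-controller traces highlight, grab, reset and X-ray tagged models.
; Grabbed models attach to an interpolated follower of a controller-mounted anchor, which slides along the pointing axis by an axis value.
; X-rayed models get a dynamic selection material and are skipped by traces, so parts behind stay selectable.
; Holding left trigger shows a wrist slider that rescales world-to-meters, controllers and widget interaction distance.
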(event Custom|RemoveXray
  ;[1 1 1] HandleXray
  (if (not (Variables|Default|GetIsModelGrabed_R))
    (CallFunction|RemoveXrayMaterial true)
    (Utilities|Array|Clear (Variables|Default|GetXrayActors))))

(event Custom|ApplyXray
  ;[1 1 1] HandleXray
  (if (not (Variables|Default|GetIsModelGrabed_R))
    (bind _out (CallFunction|GetHitLocModel true))
    (if _out
      (CallFunction|ApplyXrayMaterial))))

(event Custom|Scaling
  (params (Scale :type Float%20%28single-precision%29))
  (bind _returnvalue (|ResetSize Scale))
  ;[1 1 1] World Scale
  (if (and (not (Variables|Default|GetIsModelGrabed_R)) (Variables|Default|GetLeftTriggerPressed))
    (bind _output_get (Variables|Default|SetWorldMeter _returnvalue))
    (Class|HeadMountedDisplayFunctionLibrary|SetWorldtoMetersScale _output_get)
    (Variables|/Script/UMG.WidgetInteractionComponent|SetInteractionDistance (Variables|Default|GetWidgetInteraction) _returnvalue)
    (Default|SetWorldScale (.Right (Utilities|BPMotionControllers)) _output_get)))

(event EventBeginPlay
  ;[1 1 1] BeginPlay
  (Input|EnableInput (Game|GetPlayerController 0))
  (Utilities|FlowControl|Sequence
    (:then_0
      (CallFunction|GetInteractiveModels)
      (CallFunction|GetTeleportableSurfaces))
    (:then_1
      ;;[1 1 1] Set Motion Cotroller Pawn
      (bind _asmotion_controller_pawn (Utilities|Casting|CastToMotionControllerPawn (Game|Player|GetPlayerPawn 0)))
      (Variables|Default|SetMotionControllerPawn _asmotion_controller_pawn))
    (:then_2
      (CallFunction|InitData))))

(event EventTick
  (params (DeltaSeconds :type Float%20%28single-precision%29))
  (bind _returnvalue (Class|HeadMountedDisplayFunctionLibrary|GetWorldtoMetersScale))
  (bind _smootedattachgab (Variables|Default|GetSmootedAttachGab))
  (bind _returnvalue_2 (Math|Vector|GetForwardVector _smootedattachgab))
  (bind _returnvalue_3 (/ _returnvalue 1e+02))
  (bind _returnvalue_4 (* _returnvalue_3 -5.0))
  ;[1 1 1] set Location
  (|SetWorldMetersScale)
  (Variables|Default|SetTickDeltaSeconds DeltaSeconds)
  (if (Variables|Default|GetIsModelGrabed_R)
    (CallFunction|SmoothedTransform 15.0 (Variables|Default|GetTickDeltaSeconds))
    (Transformation|AddWorldOffset (Variables|Default|GetHardAttachGrab) (select (|Is_Close_to_Right_Hand) (* _returnvalue_2 (* (Math|Float|Clamp(Float) (stale Input|KeyboardEvents|MotionControllerRightThumbstickY AxisValue) -1.0 0.0) _returnvalue_4)) (* _returnvalue_2 (* (stale Input|KeyboardEvents|MotionControllerRightThumbstickY AxisValue) _returnvalue_4))) false false)
    (else
      (CallFunction|HighlightSelectable))))

(event Input|KeyboardEvents|MotionControllerRightThumbstickY
  (params (AxisValue :type Float%20%28single-precision%29))
  ;[1 1 1] set Location
)

(event Input|KeyboardEvents|MotionControllerRightTrigger
  (params (Key :type Key%20Structure))
  ;[1 1 1] Grab Model
  (:Pressed
    (Class|WidgetInteractionComponent|PressPointerKey (Variables|Default|GetWidgetInteraction) "LeftMouseButton")
    (if (not (Variables|Default|GetLeftTriggerPressed))
      (bind (_out _location) (CallFunction|GetHitLocModel true))
      (Variables|Default|SetHitGrabLocation _location)
      (if _out
        (Variables|Default|SetIsModelGrabed_R true)
        (Transformation|SetWorldLocation (Variables|Default|GetHardAttachGrab) (Variables|Default|GetHitGrabLocation) false false)
        (Transformation|SetWorldLocationAndRotation (Variables|Default|GetSmootedAttachGab) (Variables|Default|GetHitGrabLocation) (Transformation|GetWorldRotation (Variables|/Game/ProductViewerLogic/Blueprints/VR/BP_MotionController.BP_MotionController_C|GetMotionController (.Right (Utilities|BPMotionControllers)))) false false)
        (Transformation|AttachComponentToComponent (Variables|/Script/Engine.Actor|GetRootComponent (Variables|Default|GetHitModel)) (Variables|Default|GetSmootedAttachGab) "None" "KeepWorld" "KeepWorld" "KeepWorld" true)
        (else
          (Variables|Default|SetIsModelGrabed_R false)))))
  (:Released
    (Class|WidgetInteractionComponent|ReleasePointerKey (Variables|Default|GetWidgetInteraction) "LeftMouseButton")
    (if (Variables|Default|GetIsModelGrabed_R)
      (Transformation|DetachFromComponent (Variables|/Script/Engine.Actor|GetRootComponent (Variables|Default|GetHitModel)) "KeepWorld" "KeepWorld" "KeepWorld" true)
      (Transformation|AttachActorToActor (Variables|Default|GetHitModel) (Variables|Default|GetRootActors) "None" "KeepWorld" "KeepWorld" "KeepWorld" true)
      (Variables|Default|SetIsModelGrabed_R false)
      (else
        (Variables|Default|SetIsModelGrabed_R false)))))

(event Input|KeyboardEvents|MotionControllerLeftTrigger
  (params (Key :type Key%20Structure))
  (bind _widgetworldscale (Variables|Default|GetWidgetWorldScale))
  (bind _widgetinteraction (Variables|Default|GetWidgetInteraction))
  ;[1 1 1] WorldScale
  (:Pressed
    (Variables|Default|SetLeftTriggerPressed true)
    (Default|FadeIN _widgetworldscale)
    (Components|Activation|SetActive _widgetinteraction true false))
  (:Released
    (Variables|Default|SetLeftTriggerPressed false)
    (Default|FadeOut _widgetworldscale)
    (Components|Activation|SetActive _widgetinteraction false false)))

(event Input|KeyboardEvents|MotionControllerRightGrip1
  (params (Key :type Key%20Structure))
  ;[1 1 1] Reset model Transform
  (:Pressed
    (if (not (Variables|Default|GetIsModelGrabed_R))
      (bind _out (CallFunction|GetHitLocModel true))
      (if _out
        (CallFunction|ResettoOriginalTransform (Variables|Default|GetHitModel))))))

(fn ConstructionScript
  (|CallParentFunction))

(fn GetHitLocModel
  (params (ExcludeModels :type Boolean))
  (bind _right (Utilities|BPMotionControllers))
  (bind _motioncontroller (Variables|/Game/ProductViewerLogic/Blueprints/VR/BP_MotionController.BP_MotionController_C|GetMotionController _right))
  (bind _returnvalue (Transformation|GetWorldLocation _motioncontroller))
  (bind (_outhit _returnvalue_2) (Collision|LineTraceForObjects _returnvalue (+ _returnvalue (* (Math|Vector|GetForwardVector _motioncontroller) 1e+03)) (Utilities|Array|MakeArray "ObjectTypeQuery2" "ObjectTypeQuery1") true (select ExcludeModels (Variables|Default|GetXrayActors) 0) "None" true "(R=1.000000,G=0.000000,B=0.000000,A=1.000000)" "(R=0.000000,G=1.000000,B=0.000000,A=1.000000)" 0.2))
  (if _returnvalue_2
    (bind _output_get (LocalVariables|SetHitResult (!= (Utilities|Array|FindItem (Variables|/Script/Engine.Actor|GetTags (.HitActor (Collision|BreakHitResult _outhit))) (Utilities|Array|Get(acopy) (Variables|Default|GetInteractiveTag))) -1)))
    (if _output_get
      (Variables|Default|SetHitModel (.HitActor (Collision|BreakHitResult _outhit))))
    (else
      (LocalVariables|SetHitResult false)))
  (return (LocalVariables|GetHitResult) (.Location (Collision|BreakHitResult _outhit))))

(fn SmoothedTransform
  (params (DeltaTime :type Float%20%28single-precision%29) (InterpSpeed :type Float%20%28single-precision%29))
  (bind _hardattachgrab (Variables|Default|GetHardAttachGrab))
  (bind _smootedattachgab (Variables|Default|GetSmootedAttachGab))
  (bind _smootedattachgab_2 (Variables|Default|GetSmootedAttachGab))
  (Transformation|SetWorldLocation _smootedattachgab_2 (Math|Interpolation|VInterpTo (Transformation|GetWorldLocation _smootedattachgab) (Transformation|GetWorldLocation _hardattachgrab) DeltaTime InterpSpeed) false false)
  (Transformation|SetWorldRotation _smootedattachgab_2 (Math|Interpolation|RInterpTo (Transformation|GetWorldRotation _smootedattachgab) (Transformation|GetWorldRotation _hardattachgrab) DeltaTime InterpSpeed) false false))

(fn ResettoOriginalTransform
  (params (ItemToFind :type Actor%20Object%20Reference%20%28by%20ref%29))
  (bind _interativeactors (Variables|Default|GetInterativeActors))
  (bind _returnvalue (Utilities|Array|FindItem _interativeactors ItemToFind))
  (Transformation|SetActorLocation (Variables|Default|GetHitModel) (Utilities|Array|Get(acopy) (Variables|Default|GetInteractiveOriginalActorsLocation) _returnvalue) false false)
  (Transformation|SetActorRotation (Variables|Default|GetHitModel) (Utilities|Array|Get(acopy) (Variables|Default|GetInteractiveOriginalActorsRotation) _returnvalue)))

(fn RemoveXrayMaterial
  (params (ResetAllMaterials :type Boolean))
  (if ResetAllMaterials
    (for _array_element (Variables|Default|GetXrayActors)
      (bind _asstatic_mesh_actor (Utilities|Casting|CastToStaticMeshActor (Utilities|SelectObject _array_element (Variables|Default|GetHitModel) ResetAllMaterials)))
      (for (_ _array_index) (Rendering|Material|GetMaterials (Variables|/Script/Engine.StaticMeshActor|GetStaticMeshComponent _asstatic_mesh_actor))
        (Rendering|Material|SetMaterial (Variables|/Script/Engine.StaticMeshActor|GetStaticMeshComponent _asstatic_mesh_actor) _array_index 0)))
    (elif (Utilities|Array|ContainsItem (Variables|Default|GetXrayActors) (Variables|Default|GetHitModel))
      (Utilities|Array|RemoveItem (Variables|Default|GetXrayActors) (Variables|Default|GetHitModel))
      (bind _asstatic_mesh_actor_2 (Utilities|Casting|CastToStaticMeshActor (Utilities|SelectObject _array_element (Variables|Default|GetHitModel) ResetAllMaterials)))
      (for (_ _array_index_2) (Rendering|Material|GetMaterials (Variables|/Script/Engine.StaticMeshActor|GetStaticMeshComponent _asstatic_mesh_actor_2))
        (Rendering|Material|SetMaterial (Variables|/Script/Engine.StaticMeshActor|GetStaticMeshComponent _asstatic_mesh_actor_2) _array_index_2 0)))))

(fn ApplyXrayMaterial
  (bind _returnvalue (Rendering|Material|CreateDynamicMaterialInstance "/Game/ProductViewerLogic/Materials/Selection_Mat.Selection_Mat" :!class /Script/Engine.KismetMaterialLibrary))
  (bind _asstatic_mesh_actor (Utilities|Casting|CastToStaticMeshActor (Variables|Default|GetHitModel)))
  (for _index (range 0 (- (Rendering|Material|GetNumMaterials (Variables|/Script/Engine.StaticMeshActor|GetStaticMeshComponent _asstatic_mesh_actor)) 1))
    (Rendering|Material|SetMaterial (Variables|/Script/Engine.StaticMeshActor|GetStaticMeshComponent _asstatic_mesh_actor) _index _returnvalue))
  (Utilities|Array|Add (Variables|Default|GetXrayActors) (Variables|Default|GetHitModel)))

(fn InitData
  (bind _left (Utilities|BPMotionControllers))
  (bind _right (Utilities|BPMotionControllers))
  (bind _3d_widget_worldscale_component (Variables|Default|Get3D_Widget_WorldScale_Component))
  (bind _motioncontroller (Variables|/Game/ProductViewerLogic/Blueprints/VR/BP_MotionController.BP_MotionController_C|GetMotionController _right))
  (bind _motioncontroller_2 (Variables|/Game/ProductViewerLogic/Blueprints/VR/BP_MotionController.BP_MotionController_C|GetMotionController _left))
  (Utilities|FlowControl|Sequence
    (:then_0
      (for _array_element (Variables|Default|GetInterativeActors)
        (Utilities|Array|Add (Variables|Default|GetInteractiveOriginalActorsRotation) (Transformation|GetActorRotation _array_element))))
    (:then_1
      (for _array_element_2 (Variables|Default|GetInterativeActors)
        (Utilities|Array|Add (Variables|Default|GetInteractiveOriginalActorsLocation) (Transformation|GetActorLocation _array_element_2))))
    (:then_2
      (Utilities|Array|Clear (Variables|Default|GetXrayActors))
      (Variables|Settings|SetScaleFactor 1.0))
    (:then_3
      (Transformation|AttachComponentToComponent (Variables|Default|GetHardAttachGrab) _motioncontroller "None" "KeepWorld" "KeepWorld" "KeepWorld" true)
      (Transformation|AttachComponentToComponent (Variables|Default|GetWidgetInteraction) _motioncontroller "None" "KeepRelative" "KeepWorld" "KeepWorld" true))
    (:then_4
      (Transformation|SetWorldLocationAndRotation _3d_widget_worldscale_component (+ (Transformation|GetWorldLocation _motioncontroller_2) "20.000000,0.000000, 0") "0,180.000000, 0" false false)
      (Transformation|AttachComponentToComponent _3d_widget_worldscale_component _motioncontroller_2 "None" "KeepWorld" "KeepWorld" "KeepWorld" true)
      (bind _asworld_scale (Utilities|Casting|CastToWorldScale (UserInterface|GetUserWidgetObject (Variables|Default|Get3D_Widget_WorldScale_Component))))
      (Variables|Default|SetWidgetWorldScale _asworld_scale))))

(fn SetCustomDepth
  (params (Actor :type Actor%20Object%20Reference) (isRenderCustomDepth :type Boolean))
  (bind _asstatic_mesh_actor (Utilities|Casting|CastToStaticMeshActor Actor))
  (Rendering|SetRenderCustomDepth (Variables|/Script/Engine.StaticMeshActor|GetStaticMeshComponent _asstatic_mesh_actor) isRenderCustomDepth))

(fn HighlightSelectable
  (bind _right (Utilities|BPMotionControllers))
  (bind _motioncontroller (Variables|/Game/ProductViewerLogic/Blueprints/VR/BP_MotionController.BP_MotionController_C|GetMotionController _right))
  (bind _returnvalue (Transformation|GetWorldLocation _motioncontroller))
  (bind (_outhit _returnvalue_2) (Collision|LineTraceForObjects _returnvalue (+ _returnvalue (* (Math|Vector|GetForwardVector _motioncontroller) 1e+03)) (Utilities|Array|MakeArray "ObjectTypeQuery2" "ObjectTypeQuery1") true (Variables|Default|GetXrayActors) "None" true "(R=1.000000,G=0.000000,B=0.000000,A=1.000000)" "(R=0.000000,G=1.000000,B=0.000000,A=1.000000)" 0.2))
  (if _returnvalue_2
    (if (!= (Utilities|Array|FindItem (Variables|/Script/Engine.Actor|GetTags (.HitActor (Collision|BreakHitResult _outhit))) (Utilities|Array|Get(acopy) (Variables|Default|GetInteractiveTag))) -1)
      (Variables|Default|SetCurrentSelectable (.HitActor (Collision|BreakHitResult _outhit)))
      (if (Utilities|IsValid (Variables|Default|GetOldSelectable))
        (if (not (== (Variables|Default|GetOldSelectable) (Variables|Default|GetCurrentSelectable)))
          (CallFunction|SetCustomDepth (Variables|Default|GetOldSelectable) false)
          (bind _output_get (Variables|Default|SetOldSelectable (Variables|Default|GetCurrentSelectable)))
          (CallFunction|SetCustomDepth _output_get true))
        (else
          (bind _output_get_2 (Variables|Default|SetOldSelectable (Variables|Default|GetCurrentSelectable)))
          (CallFunction|SetCustomDepth _output_get_2 true)))
      (else
        (CallFunction|SetCustomDepth (Variables|Default|GetCurrentSelectable) false :!label _label)
        (CallFunction|SetCustomDepth (Variables|Default|GetOldSelectable) false)
        (Variables|Default|SetOldSelectable 0)))
    (else
      (goto _label))))

(event Custom|SetWorldMeter
  (params (SliderValue :type Float%20%28single-precision%29))
  (CallFunction|Scaling SliderValue))

(event Custom|SetScaleText
  (params (Value :type Float%20%28single-precision%29))
  (Rendering|Components|TextRender|SetText (Variables|/Game/ProductViewerLogic/Blueprints/Widgets/WorldScale.WorldScale_C|GetSizeHuman (Variables|Default|GetWidgetWorldScale)) (|MakeSizeText Value)))